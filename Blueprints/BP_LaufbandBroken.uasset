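; Broken conveyor belt (Laufband) actor that moves a bottle component along a spline.
; Tick advances the distance by SplineSpeed without wrapping and feeds the spline's world-space location into Bottles2's relative transform with a fixed rotation.
; The construction script repositions the actor itself at offset spline points for each MeshArray entry.
; Disconnected leftovers would spawn evenly spaced BP_Flaschen actors and loop actors along the spline by timeline.
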(event Custom|PlayTimeline
  ;[1 1 1] 3
)

(event EventTick
  (params (DeltaSeconds :type Float%20%28single-precision%29))
  ;[1 1 1] 1
  (Variables|Default|SetDistanceAlongSpline (+ (* DeltaSeconds (Variables|Default|GetSplineSpeed)) (Variables|Default|GetDistanceAlongSpline)))
  (Transformation|SetRelativeTransform (Variables|Default|GetBottles2) (Math|Transform|MakeTransform (.location (Spline|GetTransformatDistanceAlongSpline (Variables|Default|GetSpline) (Variables|Default|GetDistanceAlongSpline) "World" false)) "0.000000,-90.000000,0.000000" (Variables|/Script/Engine.SceneComponent|GetRelativeScale3D (Variables|Default|GetBottles2))) false false))

(event EventBeginPlay)

(fn ConstructionScript
  (bind _spline (Variables|Default|GetSpline))
  ;[1 1 1] 3
  (for (_ _array_index) (Variables|Default|GetMeshArray)
    (Transformation|SetActorLocationAndRotation (Spline|GetLocationatDistanceAlongSpline _spline (* (Variables|Default|GetOffset%20between%20actors) _array_index) "World") (Spline|GetRotationatDistanceAlongSpline _spline (* (Variables|Default|GetOffset%20between%20actors) _array_index) "World"))))