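; BP_Auffiller is an actor, apparently a refill point, that briefly shows a water plane to simulate spraying water.
; BeginPlay applies the WaterVisible flag to the WaterPlane, then runs a delay with nothing after it.
; The FillWater event turns the plane visible and hides it again after a short delay, with no other fill logic.
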(event Custom|FillWater
  (bind _waterplane (Variables|Default|GetWaterPlane))
  ;[1 1 1] spray water
  (bind _output_get (Variables|Default|SetWaterVisible true))
  (Rendering|SetVisibility _waterplane _output_get false)
  (Utilities|FlowControl|Delay 0.7)
  (bind _output_get_2 (Variables|Default|SetWaterVisible false))
  (Rendering|SetVisibility _waterplane _output_get_2 false))

(event EventBeginPlay
  ;[1 1 1] set invisible
  (Rendering|SetVisibility (Variables|Default|GetWaterPlane) (Variables|Default|GetWaterVisible) false)
  (Utilities|FlowControl|Delay 2.0))

(fn ConstructionScript)