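; BP_LaufbandFix is a conveyor belt actor (Laufband) that moves a bottle component (Flasche) along a spline.
; Each Tick advances a stored distance by SplineSpeed scaled by delta time, then samples Spline1 at that distance in local space.
; The bottle takes only the sampled location, keeping its scale and a fixed relative rotation.
; The distance accumulates without wrapping or resetting.
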(event EventTick
  (params (DeltaSeconds :type Float%20%28single-precision%29))
  (Variables|Default|SetDistanceAlongSpline (+ (* DeltaSeconds (Variables|Default|GetSplineSpeed)) (Variables|Default|GetDistanceAlongSpline)))
  (Transformation|SetRelativeTransform (Variables|Default|GetFlasche) (Math|Transform|MakeTransform (.location (Spline|GetTransformatDistanceAlongSpline (Variables|Default|GetSpline1) (Variables|Default|GetDistanceAlongSpline) "Local" false)) "0.000000,-90.000000,0.000000" (Variables|/Script/Engine.SceneComponent|GetRelativeScale3D (Variables|Default|GetFlasche))) false false))

(fn ConstructionScript)